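; BP_DropItemComponent is a component that drops an ammo pickup at its owner's location.
; Drop traces a short distance straight down from the owner on the Visibility channel and spawns BP_Pickup_Ammo slightly above the hit location, without checking that the trace hit.
; It passes its Type and Cout variables to the pickup as weapon ammo type and count, then destroys itself, making the drop one-shot.
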(event Custom|Drop
  (bind _returnvalue (Components|GetOwner))
  (bind _returnvalue_2 (Transformation|GetActorLocation _returnvalue))
  (bind _outhit (Collision|LineTraceByChannel _returnvalue_2 (+ _returnvalue_2 "0, 0,-100.000000") "TraceTypeQuery1" false 0 "None"))
  (Game|SpawnActorfromClass "/Game/TPS/Blueprint/InteractionEnvironment/PickupItems/BP_Pickup_Ammo.BP_Pickup_Ammo_C" (Math|Transform|MakeTransform (+ (.Location (Collision|BreakHitResult _outhit)) "0, 0,50.000000") "0,0.000000, 0") "AlwaysSpawn" 0 (Variables|Default|GetType) (Variables|Default|GetCout) 0)
  (Components|DestroyComponent))