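; BP_PlayerController is the TPS game's player controller, which creates and shows the in-game HUD widget.
; On BeginPlay it creates InGameWidget, adds it to the viewport and pushes the main sound mix.
; On Possess and UnPossess it initialises or unbinds the widget's health bar, guarded by validity checks, so the bar follows the controlled pawn.
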(event EventUnPossess
  (params (UnpossessedPawn :type Pawn%20Object%20Reference))
  (bind _ingamewidget (Variables|Default|GetInGameWidget))
  (Utilities|IsValid _ingamewidget
    (:Is%20Valid
      (Default|UnBindWidget (Variables|/Game/TPS/Blueprint/Widget/InGameWidget.InGameWidget_C|GetHealthBar _ingamewidget)))))

(event EventBeginPlay
  (bind _returnvalue (UserInterface|CreateWidget "/Game/TPS/Blueprint/Widget/InGameWidget.InGameWidget_C" self))
  (bind _output_get (Variables|Default|SetInGameWidget _returnvalue))
  (UserInterface|Viewport|AddtoViewport _output_get 0)
  (Audio|PushSoundMixModifier "/Game/TPS/Sounds/Main/MIX_Main.MIX_Main"))

(event EventPossess
  (params (PossessedPawn :type Pawn%20Object%20Reference))
  (bind _ingamewidget (Variables|Default|GetInGameWidget))
  (Utilities|IsValid _ingamewidget
    (:Is%20Valid
      (Default|InitWidget (Variables|/Game/TPS/Blueprint/Widget/InGameWidget.InGameWidget_C|GetHealthBar _ingamewidget)))))

(fn ConstructionScript)