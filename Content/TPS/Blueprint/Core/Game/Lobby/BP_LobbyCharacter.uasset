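; BP_LobbyCharacter is the lobby character, showing a player's chosen color and ready state on a skeletal mesh.
; Color changes pass from a server event to a multicast, which swaps the material in slot 0 and stores it as TrueColor.
; Remote instances reapply TrueColor on BeginPlay, and a ready multicast plays a standing rifle-equip montage.
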(event Custom|ChangeColor_OnServer
  (params (TrueColor :type Material%20Interface%20Object%20Reference))
  (CallFunction|ChangeColorMulticast TrueColor))

(event Custom|ChangeColor_Multicast
  (params (NewColor :type Material%20Interface%20Object%20Reference))
  (Rendering|Material|SetMaterial (Variables|Default|GetSkeletalMesh) 0 NewColor)
  (Variables|Default|SetTrueColor NewColor))

(event Custom|MeReady_Multicast
  (Animation|Montage|PlayMontage (Variables|Default|GetSkeletalMesh) "/Game/TPS/Characters/PlayerCharacter/Animations/Weapon/AM_Char_Equip_Rifle_Standing_Montage.AM_Char_Equip_Rifle_Standing_Montage"))

(event EventBeginPlay
  (Networking|SwitchHasAuthority
    (:Remote
      (Rendering|Material|SetMaterial (Variables|Default|GetSkeletalMesh) 0 (Variables|Default|GetTrueColor)))))

(event Collision|EventActorBeginOverlap
  (params (OtherActor :type Actor%20Object%20Reference)))

(event EventTick
  (params (DeltaSeconds :type Float%20%28single-precision%29)))

(fn ConstructionScript)