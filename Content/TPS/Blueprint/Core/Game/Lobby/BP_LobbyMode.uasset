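; Lobby game mode that tracks joined players and shares the selected level with them.
; PostLogin adds each BP_LobbyPlayerController to an array and copies the current SelectedLevel into its CurrentLevelByServer.
; UpdateLevelName stores a new selection, then loops over the stored controllers, calling UpdateLobbyWidgetOnClient on each to refresh its lobby widget.
; LaunchGame and SaveColorForPlayers are empty events.
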(event Custom|LaunchGame)

(event Custom|UpdateLevelName
  (params (SelectedLevel :type Name))
  (bind _output_get (Variables|Default|SetSelectedLevel SelectedLevel))
  (for _array_element (Variables|Default|GetPlayerController)
    (bind _asbp_lobby_player_controller (Utilities|Casting|CastToBP_LobbyPlayerController _array_element))
    (Default|UpdateLobbyWidgetonClient _asbp_lobby_player_controller _output_get)))

(event Custom|SaveColorForPlayers)

(event EventBeginPlay)

(event EventTick
  (params (DeltaSeconds :type Float%20%28single-precision%29)))

(event EventPostLogin
  (params (NewPlayer :type Player%20Controller%20Object%20Reference))
  (bind _asbp_lobby_player_controller (Utilities|Casting|CastToBP_LobbyPlayerController NewPlayer))
  (Utilities|Array|Add (Variables|Default|GetPlayerController) _asbp_lobby_player_controller)
  (Variables|/Game/TPS/Blueprint/Core/Game/Lobby/BP_LobbyPlayerController.BP_LobbyPlayerController_C|SetCurrentLevelByServer _asbp_lobby_player_controller (Variables|Default|GetSelectedLevel)))

(fn ConstructionScript)