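; BP_CharacterEnemy_1 is an enemy character variant that supplies its own animation set, including a zombie hit reaction montage.
; On BeginPlay it runs the parent logic, then assigns the hit, confusion, death, light attack and heavy attack animations.
; All other behavior comes from the parent class, as the construction script only calls its parent and Tick and overlap events are disabled.
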(event EventBeginPlay
  (|CallParentFunction)
  (Variables|Default|SetHitAnimMontage "/Game/TPS/Characters/EnemyModel1/Animations/Zombie_Reaction_Hit_Montage.Zombie_Reaction_Hit_Montage")
  (Variables|Default|SetConfusionAnim (Variables|Default|GetConfusion%20Anim))
  (Variables|Default|SetDeadsAnim (Variables|Default|GetDeads%20Anim))
  (Variables|Default|SetLightAttackAnim (Variables|Default|GetLight%20Attack%20Anim))
  (Variables|Default|SetHeavyAttackAnim (Variables|Default|GetHeavy%20Attack%20Anim)))

(event Collision|EventActorBeginOverlap
  (params (OtherActor :type Actor%20Object%20Reference))
  (|CallParentFunction OtherActor) ; This node is disabled and will not be called.\nDrag off pins to build functionality.
)

(event EventTick
  (params (DeltaSeconds :type Float%20%28single-precision%29))
  (|CallParentFunction DeltaSeconds) ; This node is disabled and will not be called.\nDrag off pins to build functionality.
)

(fn ConstructionScript
  (|CallParentFunction))