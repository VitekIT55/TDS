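; Base enemy character with melee attacks, hit reactions, death and random item drops.
; Health changes spawn damage-number actors and randomly trigger confusion, hit animations or a timed slowdown applied on Tick.
; Light and heavy attack montages sphere-trace on "Attack" notifies to damage Player-tagged actors, toggling flags behind CanMove and CanAttack.
; Death unpossesses, triggers any weapon-type drop component rolled at BeginPlay, and ragdolls after the death montage.
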(event OnHealthChange(TPSHealth)
  (params (Health :type Float%20%28single-precision%29) (Damage :type Float%20%28single-precision%29))
  (if (not (Variables|Default|GetbIsDead))
    (if (> (Math|Random|RandomFloat) (Variables|Chance|GetConfustionChance))
      (CallFunction|ConfusionEnabledTimer)
      (else
        (CallFunction|HitAnim)))
    (bind _returnvalue (Game|SpawnActorfromClass "/Game/TPS/Blueprint/InteractionEnvironment/Destruction/DisplayDamage/DisplayDamageActor.DisplayDamageActor_C" (Math|Transform|MakeTransform (+ (Transformation|GetActorLocation) (+ (Math|Vector|MakeVector (Math|Random|RandomFloatinRange -2e+01 2e+01) (Math|Random|RandomFloatinRange -2e+01 2e+01) 0.0) (Variables|Default|GetSpawnOffsetLocalDamage)))) "AlwaysSpawn" 0 0))
    (Default|InitActor _returnvalue Damage Health)
    (if (> (Math|Random|RandomFloat) (Variables|Chance|GetSlowDownSpeedChance))
      (Variables|Default|SetSlowDownSpeed true)
      (Utilities|Time|SetTimerbyEvent (delegate Custom|SlowDownDisabled) 2.0))))

(event OnDead(TPSHealth)
  (bind _deadsanim (Variables|Default|GetDeadsAnim))
  (bind _mesh (Variables|Character|GetMesh))
  (bind _returnvalue (Utilities|Array|Length _deadsanim))
  (bind _returnvalue_2 (- _returnvalue 1))
  (bind _output (Utilities|Array|Get(acopy) _deadsanim _returnvalue_2))
  (if (not (Variables|Default|GetbIsDead))
    (CallFunction|DeadEvent)
    (Utilities|IsValid _output
      (:Is%20Valid
        (Animation|Montage|PlayMontage _mesh _output
          (:OnCompleted
            (Collision|SetCollisionEnabled _mesh "PhysicsOnly")
            (Collision|SetCollisionResponsetoChannel (Variables|Collision|GetCapsuleComponent) "ECC_Pawn" "ECR_Ignore")
            (Physics|SetSimulatePhysics _mesh true)
            (Collision|SetCollisionProfileName _mesh "PhysicsActor" true :!class /Script/Engine.PrimitiveComponent)))))))

(event Custom|SlowDownDisabled
  (Variables|Default|SetSlowDownSpeed false))

(event EventBeginPlay
  (CallFunction|InitDropComponent))

(event Collision|EventActorBeginOverlap
  (params (OtherActor :type Actor%20Object%20Reference)))

(event EventTick
  (params (DeltaSeconds :type Float%20%28single-precision%29))
  (Variables|Default|SetDelta%20Time DeltaSeconds)
  (Utilities|ChangeSpeedbyHit))

(event Game|Damage|EventAnyDamage
  (params (Damage :type Float%20%28single-precision%29) (DamageType :type Damage%20Type%20Object%20Reference) (InstigatedBy :type Controller%20Object%20Reference) (DamageCauser :type Actor%20Object%20Reference))
  (if (not (Variables|Default|GetbIsDead))
    (Class|TPSHealthComponent|ChangeHealthValue (Variables|Default|GetTPSHealth) (* Damage -1.0))))

(event EventMeleeAttackHeavy
  (bind _heavyattackanim (Variables|Combat|GetHeavyAttackAnim))
  (bind _baseheavydamage (Variables|Combat|GetBaseHeavyDamage))
  (CallFunction|SetStateAttack false)
  (CallFunction|SetStateMovement false)
  (bind _notifyname (Animation|Montage|PlayMontage (Variables|Character|GetMesh) (Utilities|Array|Get(acopy) _heavyattackanim (Math|Random|RandomInteger (Utilities|Array|Length _heavyattackanim))))
    (:OnCompleted
      (CallFunction|SetStateMovement true :!label _label)
      (CallFunction|SetStateAttack true))
    (:OnInterrupted
      (goto _label))
    (:OnNotifyBegin
      (if (Utilities|Name|Equal(Name) _notifyname "Attack")
        (Utilities|MeleeTrace 5e+01 (Variables|Combat|GetEndHeavyTraceDistance) (Math|Random|RandomFloatinRange (- _baseheavydamage 1e+01) (+ _baseheavydamage 5e+01)) (Variables|Combat|GetHeavyRaduis))))))

(event EventMeleeAttackLight
  (bind _baselightdamage (Variables|Combat|GetBaseLightDamage))
  (bind _lightattackanim (Variables|Combat|GetLightAttackAnim))
  (CallFunction|SetStateAttack false)
  (bind _notifyname (Animation|Montage|PlayMontage (Variables|Character|GetMesh) (Utilities|Array|Get(acopy) _lightattackanim (Math|Random|RandomInteger (Utilities|Array|Length _lightattackanim))))
    (:OnCompleted
      (CallFunction|SetStateAttack true :!label _label))
    (:OnInterrupted
      (goto _label))
    (:OnNotifyBegin
      (if (Utilities|Name|Equal(Name) _notifyname "Attack")
        (Utilities|MeleeTrace 5e+01 1.5e+02 (Math|Random|RandomFloatinRange (- _baselightdamage 1e+01) (+ _baselightdamage 2e+01)) (Variables|Combat|GetLightRaduis))))))

(fn ConstructionScript)

(fn SetStateMovement
  (params (CanMove :type Boolean))
  (Variables|Combat|SetCanMovePawn CanMove))

(fn SetStateAttack
  (params (CanAttack :type Boolean))
  (Variables|Combat|SetCanAttackPawn CanAttack))

(fn DeadEvent
  (bind _dropcomponent (Variables|Default|GetDropComponent))
  (Pawn|UnPossess (Pawn|GetController))
  (Actor|SetLifeSpan 1e+01)
  (CallFunction|SetStateMovement false)
  (CallFunction|SetStateAttack false)
  (Variables|Default|SetbIsDead true)
  (Utilities|IsValid _dropcomponent
    (:Is%20Valid
      (Default|Drop _dropcomponent))))

(fn InitDropComponent
  (bind _returnvalue (Math|Random|RandomIntegerinRange 0 3))
  (bind _returnvalue_2 (Utilities|Select :Index _returnvalue :Option%200 "Pistol" :Option%201 "RifleType" :Option%202 "ShotGunType" :Option%203 "GrenadeLauncher"))
  (if (> (Math|Random|RandomFloat) (Variables|Chance|GetDropChance))
    (bind _returnvalue_3 (AddComponent|AddBPDropItemComponent))
    (bind _output_get (Variables|Default|SetDropComponent _returnvalue_3))
    (Variables|/Game/TPS/Blueprint/BP_DropItemComponent.BP_DropItemComponent_C|SetType _output_get _returnvalue_2)
    (Utilities|FlowControl|Sequence
      (:then_0
        (switch Utilities|FlowControl|Switch|SwitchonEWeaponType _returnvalue_2
          (:Pistol
            (LocalVariables|SetCout 12))
          (:RifleType
            (LocalVariables|SetCout 30))
          (:ShotGunType
            (LocalVariables|SetCout 5))
          (:GrenadeLauncher
            (LocalVariables|SetCout 10))))
      (:then_1
        (Variables|/Game/TPS/Blueprint/BP_DropItemComponent.BP_DropItemComponent_C|SetCout _output_get (LocalVariables|GetCout))))))

(fn ConfusionEnabledTimer
  (bind _confusionanim (Variables|Default|GetConfusionAnim))
  (CallFunction|SetStateMovement false)
  (bind _output_get (Variables|Default|SetCurrentMontage (Utilities|Array|Get(acopy) _confusionanim (Math|Random|RandomIntegerinRange 0 (- (Utilities|Array|Length _confusionanim) 1)))))
  (bind _returnvalue (Animation|GetPlayLength _output_get))
  (Utilities|Time|SetTimerbyFunctionName 0 "StunDisabledTimer" _returnvalue)
  (Animation|PlayAnimMontage (Variables|Default|GetCurrentMontage) 1.0 "None")
  (Variables|/Script/Engine.CharacterMovementComponent|SetMaxWalkSpeed (Variables|Character|GetCharacterMovement) 0.0)
  (Variables|Default|SetbIsConfused true))

(fn ConfusionDisabledTimer
  (CallFunction|SetStateMovement true)
  (Variables|/Script/Engine.CharacterMovementComponent|SetMaxWalkSpeed (Variables|Character|GetCharacterMovement) 4e+02))

(fn HitAnim
  (if (not (Variables|Default|GetbIsConfused))
    (if (> (Math|Random|RandomFloat) (Variables|Chance|GetHitAnimChance))
      (Animation|PlayAnimMontage (Variables|Default|GetHitAnimMontage) 1.0 "None"))))

(fn CanAttack
  (return (Variables|Combat|GetCanAttackPawn)))

(fn CanMove
  (return (Variables|Combat|GetCanMovePawn)))