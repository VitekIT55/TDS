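; BP_BossTurretRocket is a rocket turret that fires missiles on behalf of its owning boss character.
; A looping timer started on BeginPlay checks the boss's health and plays the Shoot timeline while it is alive, clearing itself otherwise.
; The timeline's Shoot event spawns a BP_ProjectileMissleTurret ahead of the Arrow component, owned by the boss and initialized with dark rocket mesh, effects and radial explosion damage.
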(event Custom|FireRocket
  (bind _returnvalue (Components|GetOwner))
  (bind _arrow (Variables|Default|GetArrow))
  (bind _asbp_character_enemy_boss (Utilities|Casting|CastToBP_CharacterEnemy_Boss _returnvalue))
  (bind _returnvalue_2 (Class|TPSHealthComponent|GetCurrentHealth (Variables|/Game/TPS/Blueprint/EnemyCharacter/BP_CharacterEnemy_Base.BP_CharacterEnemy_Base_C|GetTPSHealth _asbp_character_enemy_boss)))
  (if (> _returnvalue_2 0.0)
    (Timeline|Shoot PlayFromStart
      (:Shoot
        (bind _returnvalue_3 (Game|SpawnActorfromClass "/Game/TPS/Blueprint/EnemyCharacter/BossTurret/BP_ProjectileMissleTurret.BP_ProjectileMissleTurret_C" (Math|Transform|MakeTransform (+ (* (Math|Vector|GetForwardVector _arrow) 1e+02) (Transformation|GetWorldLocation _arrow)) (Transformation|GetWorldRotation _arrow)) "AlwaysSpawn" _returnvalue 0))
        (Class|ProjectileDefault|InitProjectile _returnvalue_3 (Utilities|Struct|MakeProjectileInfo "/Game/TPS/Blueprint/EnemyCharacter/BossTurret/BP_ProjectileMissleTurret.BP_ProjectileMissleTurret_C" "/Game/TPS/Items/GameActor/Weapons/Weapons/Darkness_RocketLauncher_Ammo.Darkness_RocketLauncher_Ammo" (Math|Transform|MakeTransform "0, 0, 0" "0, 0, 0" "4.000000,4.000000,4.000000") "/Game/TPS/Items/GameActor/Weapons/FX/Particles/P_RocketLauncher_Trail_Dark.P_RocketLauncher_Trail_Dark" "0.000000,0.000000,0.000000|0.000000,0.000000,0.000000|1.000000,1.000000,1.000000" 1.0 2e+01 5e+02 1e+03 "SurfaceType_Default" 0 "SurfaceType_Default" 0 "/Game/TPS/Items/GameActor/Weapons/FX/Particles/P_RocketLauncher_Explosion_Dark.P_RocketLauncher_Explosion_Dark" "/Game/TPS/Items/GameActor/Weapons/Sound/RocketLauncher/RocketLauncher_Explosion_Cue.RocketLauncher_Explosion_Cue" 4e+02 2e+02 6e+01))))
    (else
      (Utilities|Time|ClearandInvalidateTimerbyHandle (Variables|Default|GetFireRocket_HandleTimer)))))

(event EventBeginPlay
  (bind _returnvalue (Utilities|Time|SetTimerbyEvent (delegate Custom|FireRocket) 3.0 true))
  (Variables|Default|SetFireRocket_HandleTimer _returnvalue))

(event Collision|EventActorBeginOverlap
  (params (OtherActor :type Actor%20Object%20Reference)))

(event EventTick
  (params (DeltaSeconds :type Float%20%28single-precision%29)))

(fn ConstructionScript)