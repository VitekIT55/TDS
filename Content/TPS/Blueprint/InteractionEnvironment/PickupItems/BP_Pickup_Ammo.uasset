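; Ammo pickup for the TPS inventory system that gives a configurable amount of ammo for one weapon type to an overlapping character.
; On BeginPlay, InitActor picks the mesh and spinner particle matching the weapon type, destroying either component if its asset is invalid.
; The parent's OverlapCharacter event supplies the inventory, which is checked for whether it can take that ammo before the count is added and PickupSuccess runs.
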(event Custom|OverlapCharacter
  (params (ToInventory :type TPS%20Inventory%20Component%20Object%20Reference))
  (bind _weapontypeammo (Variables|Default|GetWeaponTypeAmmo))
  (|CallParentFunction ToInventory)
  (bind _returnvalue (Class|TPSInventoryComponent|CheckCanTakeAmmo ToInventory _weapontypeammo))
  (if _returnvalue
    (Class|TPSInventoryComponent|AmmoSlotChangeValue ToInventory _weapontypeammo (Variables|Default|GetCout))
    (CallFunction|PickupSuccess)))

(event EventBeginPlay
  (|CallParentFunction)
  (CallFunction|InitActor))

(event Collision|EventActorBeginOverlap
  (params (OtherActor :type Actor%20Object%20Reference))
  (|CallParentFunction OtherActor) ; This node is disabled and will not be called.\nDrag off pins to build functionality.
)

(event EventTick
  (params (DeltaSeconds :type Float%20%28single-precision%29))
  (|CallParentFunction DeltaSeconds) ; This node is disabled and will not be called.\nDrag off pins to build functionality.
)

(fn ConstructionScript
  (|CallParentFunction))

(fn InitActor
  (bind _weapontypeammo (Variables|Default|GetWeaponTypeAmmo))
  (bind _particlesystem (Variables|Default|GetParticleSystem))
  (bind _staticmesh (Variables|Default|GetStaticMesh))
  (bind _returnvalue (Utilities|Select :Index _weapontypeammo :Pistol "/Game/TPS/WeaponItems/GameActor/Weapons/Pickups/Darkness_Pistol_Pickup.Darkness_Pistol_Pickup" :RifleType "/Game/TPS/WeaponItems/GameActor/Weapons/Pickups/Darkness_AssaultRifle_Pickup.Darkness_AssaultRifle_Pickup" :ShotGunType "/Game/TPS/WeaponItems/GameActor/Weapons/Pickups/Darkness_Shotgun_Pickup.Darkness_Shotgun_Pickup" :GrenadeLauncher "/Game/TPS/WeaponItems/GameActor/Weapons/Pickups/Darkness_GrenadeLauncher_Pickup.Darkness_GrenadeLauncher_Pickup"))
  (bind _returnvalue_2 (Utilities|Select :Index _weapontypeammo :Pistol "/Game/TPS/Recurces/FX_Effects/Particles/InteractionEnvironment/P_Spinner_Ammo_Pistol.P_Spinner_Ammo_Pistol" :RifleType "/Game/TPS/Recurces/FX_Effects/Particles/InteractionEnvironment/P_Spinner_Ammo_Rifle.P_Spinner_Ammo_Rifle" :ShotGunType "/Game/TPS/Recurces/FX_Effects/Particles/InteractionEnvironment/P_Spinner_Ammo_Shotgun.P_Spinner_Ammo_Shotgun" :GrenadeLauncher "/Game/TPS/Recurces/FX_Effects/Particles/InteractionEnvironment/P_Spinner_Ammo_GrenadeLauncher.P_Spinner_Ammo_GrenadeLauncher"))
  (Utilities|FlowControl|Sequence
    (:then_0
      (Utilities|IsValid _returnvalue
        (:Is%20Valid
          (Components|StaticMesh|SetStaticMesh _staticmesh _returnvalue)
          (Transformation|SetRelativeScale3D _staticmesh "1.500000,1.500000,1.500000"))
        (:Is%20Not%20Valid
          (Components|DestroyComponent _staticmesh))))
    (:then_1
      (Utilities|IsValid _returnvalue_2
        (:Is%20Valid
          (Effects|Components|ParticleSystem|SetTemplate _particlesystem _returnvalue_2))
        (:Is%20Not%20Valid
          (Components|DestroyComponent _particlesystem))))))